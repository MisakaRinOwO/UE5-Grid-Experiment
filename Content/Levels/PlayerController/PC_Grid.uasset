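; Player controller for a grid pathfinding level, showing the mouse cursor and moving the grid pawn as a camera.
; BeginPlay caches the pawn, adds the grid Enhanced Input mapping context and finds the GridManager actor.
; Select, start, goal and run inputs toggle obstacles, set endpoints or call FindPath on the manager.
; RunRaytrace traces from the cursor on the Visibility channel and converts the hit to a grid coordinate, validated before use.
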(event `self.ReceiveBeginPlay`
  (bind _returnvalue (subsystem `EnhancedInputLocalPlayerSubsystem`))
  (set `self.bShowMouseCursor` true)
  (bind _asbp_grid_pawn (cast `/Game/Levels/Pawn/BP_GridPawn` (`self.K2_GetPawn`)))
  (set `self.Controlled Pawn` _asbp_grid_pawn)
  (`/Engine/EditorBlueprintResources/StandardMacros.IsValid` _returnvalue
    (:`Is Valid`
      (`EnhancedInputSubsystemInterface.AddMappingContext` _returnvalue "/Game/Levels/Input/IMC_Grid.IMC_Grid" 0 (struct))
      (bind _returnvalue_2 (`GameplayStatics.GetActorOfClass` "/Script/GridExperiment.GridManager"))
      (`/Engine/EditorBlueprintResources/StandardMacros.IsValid` _returnvalue_2
        (:`Is Valid`
          (set `self.Grid Manager` _returnvalue_2))))))

(event `EnhancedInput|/Game/Levels/Input/InputActions/IA_GridMove`
  (params (ActionValue :type "Vector2D Structure") (ElapsedSeconds :type "Float (double-precision)") (TriggeredSeconds :type "Float (double-precision)") (InputAction :type "InputAction Object Reference" :default "/Game/Levels/Input/InputActions/IA_GridMove.IA_GridMove"))
  (:`Triggered`
    ;[0.15 0.15 0.15 0.502] Camera Logic
    (`Pawn.AddMovementInput` (`self.Controlled Pawn`) (`self.Right Unit`) ActionValue_X false)
    (`Pawn.AddMovementInput` (`self.Controlled Pawn`) (`self.Up Unit`) ActionValue_Y false)))

(event `EnhancedInput|/Game/Levels/Input/InputActions/IA_GridSelect`
  (params (ActionValue :type Boolean) (ElapsedSeconds :type "Float (double-precision)") (TriggeredSeconds :type "Float (double-precision)") (InputAction :type "InputAction Object Reference" :default "/Game/Levels/Input/InputActions/IA_GridSelect.IA_GridSelect"))
  (:`Triggered`
    (bind _grid_manager (`self.Grid Manager`)
      (:`then`
        (bind (_grid_coord _return_value) (`self.Run Raytrace`))
        (if _return_value
          (if (`GridManager.IsValidCoord` _grid_manager _grid_coord)
            (`GridManager.ToggleObstacle` _grid_manager _grid_coord))))
      (:`else`))))

(event `EnhancedInput|/Game/Levels/Input/InputActions/IA_SetStartGrid`
  (params (ActionValue :type Boolean) (ElapsedSeconds :type "Float (double-precision)") (TriggeredSeconds :type "Float (double-precision)") (InputAction :type "InputAction Object Reference" :default "/Game/Levels/Input/InputActions/IA_SetStartGrid.IA_SetStartGrid"))
  (:`Triggered`
    (bind _grid_manager (`self.Grid Manager`)
      (:`then`
        (bind (_grid_coord _return_value) (`self.Run Raytrace`))
        (if _return_value
          (if (`GridManager.IsValidCoord` _grid_manager _grid_coord)
            (`GridManager.SetStartCoord` _grid_manager _grid_coord))))
      (:`else`))))

(event `EnhancedInput|/Game/Levels/Input/InputActions/IA_SetGoalGrid`
  (params (ActionValue :type Boolean) (ElapsedSeconds :type "Float (double-precision)") (TriggeredSeconds :type "Float (double-precision)") (InputAction :type "InputAction Object Reference" :default "/Game/Levels/Input/InputActions/IA_SetGoalGrid.IA_SetGoalGrid"))
  (:`Triggered`
    (bind _grid_manager (`self.Grid Manager`)
      (:`then`
        (bind (_grid_coord _return_value) (`self.Run Raytrace`))
        (if _return_value
          (if (`GridManager.IsValidCoord` _grid_manager _grid_coord)
            (`GridManager.SetGoalCoord` _grid_manager _grid_coord))))
      (:`else`))))

(event `EnhancedInput|/Game/Levels/Input/InputActions/IA_RunPathfinding`
  (params (ActionValue :type Boolean) (ElapsedSeconds :type "Float (double-precision)") (TriggeredSeconds :type "Float (double-precision)") (InputAction :type "InputAction Object Reference" :default "/Game/Levels/Input/InputActions/IA_RunPathfinding.IA_RunPathfinding"))
  (:`Triggered`
    (bind _grid_manager (`self.Grid Manager`)
      (:`then`
        (`GridManager.FindPath` _grid_manager))
      (:`else`))))

(fn `Run Raytrace`
  (returns (`Grid Coord` :type "GridCoord Structure") (`Return Value` :type Boolean))
  (bind (_locationx _locationy) (`self.GetMousePosition`))
  (bind (_worldposition _worlddirection) (`GameplayStatics.DeprojectScreenToWorld` self (`KismetMathLibrary.MakeVector2D` _locationx _locationy)))
  (`self.Grid Manager`
    (:`then`
      (bind (_outhit _returnvalue) (`KismetSystemLibrary.LineTraceSingle` _worldposition (+ _worldposition (* _worlddirection (`GridManager.TraceDistance` (`self.Grid Manager`)))) "TraceTypeQuery1"))
      (if _returnvalue
        (return (`GridManager.WorldToGrid` (`self.Grid Manager`) (`KismetMathLibrary.MakeVector` (.x (`.Location` (`GameplayStatics.BreakHitResult` _outhit))) (.y (`.Location` (`GameplayStatics.BreakHitResult` _outhit))))) true)
        (else
          (return (struct) false))))
    (:`else`)))

(fn `UserConstructionScript`)