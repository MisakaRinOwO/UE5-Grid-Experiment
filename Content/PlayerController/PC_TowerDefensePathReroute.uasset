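; Player controller for a grid tower-defense pathfinding demo, where the player edits obstacles, start and goal cells with the mouse.
; Begin play adds the grid input context, configures the GridManager and shows a tooltip widget; move input pans the grid pawn.
; Clicks trace from the cursor to a grid coordinate, apply the edit, then re-run FindPath on demand.
; An obstacle that would block the path is toggled back with a printed warning.
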(event `self.ReceiveBeginPlay`
  (bind _returnvalue (subsystem `EnhancedInputLocalPlayerSubsystem`))
  (`|ExecutionSequence`
    (:`then_0`
      (set `self.bShowMouseCursor` true)
      (bind _asbp_grid_pawn (cast `/Game/Pawn/BP_GridPawn` (`self.K2_GetPawn`)))
      (set `self.Controlled Pawn` _asbp_grid_pawn)
      (`/Engine/EditorBlueprintResources/StandardMacros.IsValid` _returnvalue
        (:`Is Valid`
          (`EnhancedInputSubsystemInterface.AddMappingContext` _returnvalue "/Game/Input/IMC_Grid.IMC_Grid" 0 (struct))
          (bind _returnvalue_2 (`GameplayStatics.GetActorOfClass` "/Script/GridExperiment.GridManager"))
          (`/Engine/EditorBlueprintResources/StandardMacros.IsValid` _returnvalue_2
            (:`Is Valid`
              (bind _output_get (set `self.Grid Manager` _returnvalue_2))
              (set `GridManager.bDrawCellCostText` false _output_get)
              ; Disable movement range debug
              (set `GridManager.MovementBudget` 0.0 _output_get))))))
    (:`then_1`
      (bind _returnvalue_3 (`|CreateWidget` "/Game/UI/W_TooltipTowerDefense.W_TooltipTowerDefense_C"))
      (`UserWidget.AddToViewport` _returnvalue_3 0))))

(event `EnhancedInput|/Game/Input/InputActions/IA_GridMove`
  (params (ActionValue :type "Vector2D Structure") (ElapsedSeconds :type "Float (double-precision)") (TriggeredSeconds :type "Float (double-precision)") (InputAction :type "InputAction Object Reference" :default "/Game/Input/InputActions/IA_GridMove.IA_GridMove"))
  (:`Triggered`
    ;[0.15 0.15 0.15 0.502] Camera Logic
    (`Pawn.AddMovementInput` (`self.Controlled Pawn`) (`self.Right Unit`) ActionValue_X false)
    (`Pawn.AddMovementInput` (`self.Controlled Pawn`) (`self.Up Unit`) ActionValue_Y false)))

(event `EnhancedInput|/Game/Input/InputActions/IA_GridLeft`
  (params (ActionValue :type Boolean) (ElapsedSeconds :type "Float (double-precision)") (TriggeredSeconds :type "Float (double-precision)") (InputAction :type "InputAction Object Reference" :default "/Game/Input/InputActions/IA_GridLeft.IA_GridLeft"))
  (:`Triggered`
    ; Get clicked grid and validate
    (bind _grid_manager (`self.Grid Manager`)
      (:`then`
        (bind (_grid_coord _return_value) (`self.Run Raytrace`))
        (if _return_value
          (if (`GridManager.IsValidCoord` _grid_manager _grid_coord)
            ; Perform grid operation
            (bind _returnvalue (`GridManager.ToggleObstacle` _grid_manager _grid_coord))
            (if _returnvalue
              (set `self.Pending Toggle Obstacle` _grid_coord)
              ; On demand re-calculate path
              (bind _path_is_valid (`self.Run Findpath`))
              ; Fallback if obstacle blocks path
              (if (not _path_is_valid)
                (`GridManager.ToggleObstacle` _grid_manager _grid_coord)
                (`KismetSystemLibrary.PrintString` "Cannot set grid as obstacle, path will be blocked.")
                (`self.Run Findpath`))))))
      (:`else`))))

(event `EnhancedInput|/Game/Input/InputActions/IA_SetStartGrid`
  (params (ActionValue :type Boolean) (ElapsedSeconds :type "Float (double-precision)") (TriggeredSeconds :type "Float (double-precision)") (InputAction :type "InputAction Object Reference" :default "/Game/Input/InputActions/IA_SetStartGrid.IA_SetStartGrid"))
  (:`Triggered`
    ; Get clicked grid and validate
    (bind _grid_manager (`self.Grid Manager`)
      (:`then`
        (bind (_grid_coord _return_value) (`self.Run Raytrace`))
        (if _return_value
          (if (`GridManager.IsValidCoord` _grid_manager _grid_coord)
            ; Perform grid operation
            (bind _returnvalue (`GridManager.SetStartCoord` _grid_manager _grid_coord))
            (if _returnvalue
              ; On demand re-calculate path
              (`self.Run Findpath`)))))
      (:`else`))))

(event `EnhancedInput|/Game/Input/InputActions/IA_SetGoalGrid`
  (params (ActionValue :type Boolean) (ElapsedSeconds :type "Float (double-precision)") (TriggeredSeconds :type "Float (double-precision)") (InputAction :type "InputAction Object Reference" :default "/Game/Input/InputActions/IA_SetGoalGrid.IA_SetGoalGrid"))
  (:`Triggered`
    ; Get clicked grid and validate
    (bind _grid_manager (`self.Grid Manager`)
      (:`then`
        (bind (_grid_coord _return_value) (`self.Run Raytrace`))
        (if _return_value
          (if (`GridManager.IsValidCoord` _grid_manager _grid_coord)
            ; Perform grid operation
            (bind _returnvalue (`GridManager.SetGoalCoord` _grid_manager _grid_coord))
            (if _returnvalue
              ; On demand re-calculate path
              (`self.Run Findpath`)))))
      (:`else`))))

(event `EnhancedInput|/Game/Input/InputActions/IA_RunPathfinding`
  (params (ActionValue :type Boolean) (ElapsedSeconds :type "Float (double-precision)") (TriggeredSeconds :type "Float (double-precision)") (InputAction :type "InputAction Object Reference" :default "/Game/Input/InputActions/IA_RunPathfinding.IA_RunPathfinding"))
  (:`Triggered`
    (bind _grid_manager (`self.Grid Manager`)
      (:`then`
        (`GridManager.FindPath` _grid_manager))
      (:`else`))))

(fn `Run Findpath`
  (returns (`Path Is Valid` :type Boolean))
  (bind _grid_manager (`self.Grid Manager`)
    (:`then`
      (bind _returnvalue (`GridManager.FindPath` _grid_manager))
      (return _returnvalue))
    (:`else`)))

(fn `Run Raytrace`
  (returns (`Grid Coord` :type "GridCoord Structure") (`Return Value` :type Boolean))
  (bind (_locationx _locationy) (`self.GetMousePosition`))
  (bind (_worldposition _worlddirection) (`GameplayStatics.DeprojectScreenToWorld` self (`KismetMathLibrary.MakeVector2D` _locationx _locationy)))
  (`self.Grid Manager`
    (:`then`
      (bind (_outhit _returnvalue) (`KismetSystemLibrary.LineTraceSingle` _worldposition (+ _worldposition (* _worlddirection (`GridManager.TraceDistance` (`self.Grid Manager`)))) "TraceTypeQuery1"))
      (if _returnvalue
        (return (`GridManager.WorldToGrid` (`self.Grid Manager`) (`KismetMathLibrary.MakeVector` (.x (`.Location` (`GameplayStatics.BreakHitResult` _outhit))) (.y (`.Location` (`GameplayStatics.BreakHitResult` _outhit))))) true)
        (else
          (return (struct) false))))
    (:`else`)))

(fn `UserConstructionScript`)