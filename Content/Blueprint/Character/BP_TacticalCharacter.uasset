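; Tactical character that walks along a path of grid cells supplied by a grid manager.
; Starting a move toggles the first cell's occupancy and converts the path to world points, offset by the height captured at BeginPlay.
; Tick steps the actor toward each point at constant speed, facing its travel direction and snapping within an acceptance distance.
; Finishing fires the movement-finished dispatcher and registers the character on the last cell.
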(event `self.ReceiveBeginPlay`
  (bind (_returnvalue_x _returnvalue_y _returnvalue_z) (`KismetMathLibrary.BreakVector` (`self.K2_GetActorLocation`)))
  (set `self.MoveZOffset` _returnvalue_z))

(event `self.ReceiveTick`
  (params (DeltaSeconds :type "Float (single-precision)"))
  (`self.Is Moving Along Path`
    (:`then`
      (`self.Move Along Path Tick` DeltaSeconds))
    (:`else`)))

(fn `Convert Path to World Location`
  (returns (`Out Array` :type "Array of Vector Structure"))
  (for _array_element (`self.Current Path`)
    (bind (_returnvalue_x _returnvalue_y _returnvalue_z) (`KismetMathLibrary.BreakVector` (`GridManager.GridToWorld` (`self.Grid Manager`) _array_element)))
    (`KismetArrayLibrary.Array_Add` (`local.Out Array`) (`KismetMathLibrary.MakeVector` _returnvalue_x _returnvalue_y (+ _returnvalue_z (`self.MoveZOffset`)))))
  (return (`local.Out Array`)))

(fn `Finish Path Movement`
  (bind _current_path (`self.Current Path`))
  (set `self.Is Moving Along Path` false)
  (`self.On Path Movement Finished`)
  (`GridManager.AssignGridCellCharacterAndUpdateOccupancy` (`self.Grid Manager`) (`|GetArrayItem` (`GridManager.Cells` (`self.Grid Manager`)) (`GridManager.CoordToIndex` (`self.Grid Manager`) (`|GetArrayItem` _current_path (- (`KismetArrayLibrary.Array_Length` _current_path) 1)))) self))

(fn `Move Along Path Tick`
  (params (`Delta Seconds` :type "Float (double-precision)"))
  (locals (`Current Location` :type "Vector Structure") (`Target Location` :type "Vector Structure") (Direction :type "Vector Structure") (Distance :type "Float (double-precision)") (`DirectionNormalized ` :type "Vector Structure") (`Step Distance` :type "Float (double-precision)") (`New Location` :type "Vector Structure"))
  (if (`KismetArrayLibrary.Array_IsValidIndex` (`self.World Location Array`) (`self.Current Path Index`))
    (set `local.Current Location` (`self.K2_GetActorLocation`))
    (set `local.Target Location` (`|GetArrayItem` (`self.World Location Array`) (`self.Current Path Index`)))
    (bind _output_get (set `local.Direction` (- (`local.Target Location`) (`local.Current Location`))))
    (bind _output_get_2 (set `local.Distance` (`KismetMathLibrary.VSize` _output_get)))
    (`/Engine/EditorBlueprintResources/StandardMacros.CompareFloat` _output_get_2 (`self.Acceptance Distance`)
      (:`>`
        (`|ExecutionSequence` :!label _label
          (:`then_0`
            (set `local.DirectionNormalized ` (`KismetMathLibrary.Normal` (`local.Direction`))))
          (:`then_1`
            (`self.K2_SetActorRotation` (`KismetMathLibrary.MakeRotFromX` (`local.DirectionNormalized `))))
          (:`then_2`
            (set `local.Step Distance` (* (`self.Move Speed`) (`local.Delta Seconds`))))
          (:`then_3`
            (bind _output_get_3 (set `local.New Location` (+ (`local.Current Location`) (* (`local.DirectionNormalized `) (`KismetMathLibrary.FMin` (`local.Step Distance`) (`local.Distance`))))))
            (`self.K2_SetActorLocation` _output_get_3))))
      (:`==`
        (`self.K2_SetActorLocation` (`local.Target Location`) :!label _label_2)
        (bind _result (`/Engine/EditorBlueprintResources/StandardMacros.IncrementInt` (`self.Current Path Index`))
          (:`  `
            (`/Engine/EditorBlueprintResources/StandardMacros.CompareInt` _result (`KismetArrayLibrary.Array_Length` (`self.World Location Array`))
              (:`>`
                _)
              (:`==`
                _)
              (:`<`
                (goto _label)))
            (`self.Finish Path Movement`))))
      (:`<`
        (goto _label_2)))
    (else
      (`self.Finish Path Movement`))))

(fn `Start Move Along Path`
  (params (Path :type "Array of GridCoord Structure") (`Grid Manager` :type "GridManager Object Reference"))
  (if (> (`KismetArrayLibrary.Array_Length` (`GridManager.CurrentPath` `Grid Manager`)) 1)
    (set `self.Current Path Index` 1)
    (`KismetArrayLibrary.Array_Clear` (`self.Current Path`))
    (set `self.Current Path` (`GridManager.CurrentPath` (`self.Grid Manager`)))
    (`GridManager.ToggleGridCellOccupied` (`self.Grid Manager`) (`|GetArrayItem` (`GridManager.Cells` (`self.Grid Manager`)) (`GridManager.CoordToIndex` (`self.Grid Manager`) (`|GetArrayItem` (`GridManager.CurrentPath` (`self.Grid Manager`))))))
    (`KismetArrayLibrary.Array_Clear` (`self.World Location Array`))
    (bind _out_array (`self.Convert Path to World Location`))
    (set `self.World Location Array` _out_array)
    (set `self.Is Moving Along Path` true)
    (else
      (`self.On Path Movement Finished`))))

(fn `UserConstructionScript`)