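; Player controller for a tactical grid prototype, moving the camera pawn and cycling Terrain Editor, Move Range and Skill Attack modes.
; Cursor traces become grid coordinates for GridManager.
; Terrain clicks cycle cell cost or spawn and remove units; Move Range clicks select units and start path movement, setting an interaction lock until movement finishes.
; Skill Attack only previews the selected unit's first skill on Tick, from its cell toward the hovered one.
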(event `self.ReceiveBeginPlay`
  (bind _returnvalue (subsystem `EnhancedInputLocalPlayerSubsystem`))
  (`|ExecutionSequence`
    (:`then_0`
      (set `self.bShowMouseCursor` true)
      (bind _asbp_grid_pawn (cast `/Game/Blueprint/Pawn/BP_GridPawn` (`self.K2_GetPawn`)))
      (set `self.Controlled Pawn` _asbp_grid_pawn)
      (`/Engine/EditorBlueprintResources/StandardMacros.IsValid` _returnvalue
        (:`Is Valid`
          (`EnhancedInputSubsystemInterface.AddMappingContext` _returnvalue "/Game/Input/IMC_Grid.IMC_Grid" 0 (struct))
          (bind _returnvalue_2 (`GameplayStatics.GetActorOfClass` "/Script/GridExperiment.GridManager"))
          (`/Engine/EditorBlueprintResources/StandardMacros.IsValid` _returnvalue_2
            (:`Is Valid`
              (bind _output_get (set `self.Grid Manager` _returnvalue_2))
              (set `GridManager.bDrawCellCostText` true _output_get))))))
    (:`then_1`
      (bind _returnvalue_3 (`|CreateWidget` "/Game/UI/W_TooltipTacticalMovement.W_TooltipTacticalMovement_C"))
      (`UserWidget.AddToViewport` _returnvalue_3 0)
      (set `self.UI` _returnvalue_3))))

(event `EnhancedInput|/Game/Input/InputActions/IA_GridMove`
  (params (ActionValue :type "Vector2D Structure") (ElapsedSeconds :type "Float (double-precision)") (TriggeredSeconds :type "Float (double-precision)") (InputAction :type "InputAction Object Reference" :default "/Game/Input/InputActions/IA_GridMove.IA_GridMove"))
  (:`Triggered`
    ;[0.15 0.15 0.15 0.502] Camera Logic
    (`Pawn.AddMovementInput` (`self.Controlled Pawn`) (`self.Right Unit`) ActionValue_X false)
    (`Pawn.AddMovementInput` (`self.Controlled Pawn`) (`self.Up Unit`) ActionValue_Y false)))

(event `EnhancedInput|/Game/Input/InputActions/IA_GridLeft`
  (params (ActionValue :type Boolean) (ElapsedSeconds :type "Float (double-precision)") (TriggeredSeconds :type "Float (double-precision)") (InputAction :type "InputAction Object Reference" :default "/Game/Input/InputActions/IA_GridLeft.IA_GridLeft"))
  (:`Triggered`
    (`self.Interaction Lock`
      (:`then`)
      (:`else`
        (switch `/Game/Blueprint/Enum/E_WeightedTerrianMode` (`self.Current Mode`)
          (:`NewEnumerator0`
            ; Get clicked grid and validate
            (bind _grid_manager (`self.Grid Manager`)
              (:`then`
                (bind (_grid_coord _return_value) (`self.Run Raytrace`))
                (if _return_value
                  (if (`GridManager.IsValidCoord` _grid_manager _grid_coord)
                    ; Perform grid operation
                    (`GridManager.CycleGridCost` _grid_manager _grid_coord))))
              (:`else`)))
          (:`NewEnumerator1`
            ; Get clicked grid and validate
            (bind _grid_manager_2 (`self.Grid Manager`)
              (:`then`
                (bind (_grid_coord_2 _return_value_2) (`self.Run Raytrace`))
                (if _return_value_2
                  (bind (_outcell _returnvalue) (`GridManager.TryGetGridCell` _grid_manager_2 _grid_coord_2))
                  (if _returnvalue
                    (bind (_coord _bblocked _movecost _movecostlistindex _bisoccupied _occupyingcharacter) (break `GridCell` _outcell))
                    (if _bisoccupied
                      (bind _asbp_tactical_character (cast `/Game/Blueprint/Character/BP_TacticalCharacter` _occupyingcharacter))
                      (bind _output_get (set `self.Selected Character` _asbp_tactical_character))
                      (set `GridManager.MovementBudget` (`/Game/Blueprint/DataAsset/Unit/DA_Unit.Movement Budget` (`/Game/Blueprint/Character/BP_TacticalCharacter.Character Preset` _output_get)) (`self.Grid Manager`))
                      (bind _returnvalue_2 (`GridManager.SetStartCoord` (`self.Grid Manager`) _coord))
                      (if _returnvalue_2
                        (add `/Game/Blueprint/Character/BP_TacticalCharacter.On Path Movement Finished` (`self.Selected Character`) (delegate `On Movement Finished`))
                        (else
                          (`KismetSystemLibrary.PrintString` "Cannot select grid: Target grid is obstacle")))
                      (else
                        (`KismetSystemLibrary.PrintString` "Cannot select grid: Target grid has no unit."))))))
              (:`else`))))))))

(event `On Movement Finished`
  (`GridManager.RemoveStartAndGoalCoord` (`self.Grid Manager`))
  (set `self.Selected Character` null)
  (set `self.Interaction Lock` false))

(event `EnhancedInput|/Game/Input/InputActions/IA_GridRight`
  (params (ActionValue :type Boolean) (ElapsedSeconds :type "Float (double-precision)") (TriggeredSeconds :type "Float (double-precision)") (InputAction :type "InputAction Object Reference" :default "/Game/Input/InputActions/IA_GridRight.IA_GridRight"))
  (:`Triggered`
    (`self.Interaction Lock`
      (:`then`)
      (:`else`
        (set `self.Interacting Cell` (struct))
        (switch `/Game/Blueprint/Enum/E_WeightedTerrianMode` (`self.Current Mode`)
          (:`NewEnumerator0`
            ; Get clicked grid and validate
            (bind _grid_manager (`self.Grid Manager`)
              (:`then`
                (bind (_grid_coord _return_value) (`self.Run Raytrace`))
                (if _return_value
                  (bind (_outcell _returnvalue) (`GridManager.TryGetGridCell` _grid_manager _grid_coord))
                  (if _returnvalue
                    (bind _output_get (set `self.Interacting Cell` _outcell))
                    (if (`.bIsOccupied` (break `GridCell` _output_get))
                      ; Destroy unit and reset cell stat
                      (`self.K2_DestroyActor` (`.OccupyingCharacter` (break `GridCell` _output_get)))
                      (`GridManager.AssignGridCellCharacterAndUpdateOccupancy` (`self.Grid Manager`) (`self.Interacting Cell`) null)
                      (set `self.Selected Character` null)
                      (else
                        (bind (_returnvalue_x _returnvalue_y _returnvalue_z) (`KismetMathLibrary.BreakVector` (`GridManager.GridToWorld` (`self.Grid Manager`) (break `GridCell` _output_get))))
                        ; Create unit and update cell stat
                        (bind _returnvalue_2 (`|SpawnActorFromClass` "/Game/Blueprint/Character/BP_TacticalCharacter.BP_TacticalCharacter_C" (`KismetMathLibrary.MakeTransform` (`KismetMathLibrary.MakeVector` _returnvalue_x _returnvalue_y (+ _returnvalue_z 90.0))) "Undefined" "MultiplyWithRoot" null "/Game/Blueprint/DataAsset/Unit/DA_Mage.DA_Mage" (`self.Grid Manager`) null))
                        (`GridManager.AssignGridCellCharacterAndUpdateOccupancy` (`self.Grid Manager`) (`self.Interacting Cell`) _returnvalue_2)))
                    (`GridManager.RemoveStartAndGoalCoord` (`self.Grid Manager`)))))
              (:`else`)))
          (:`NewEnumerator1`
            ; Get clicked grid and validate
            (bind _grid_manager_2 (`self.Grid Manager`)
              (:`then`
                (bind (_grid_coord_2 _return_value_2) (`self.Run Raytrace`))
                (if _return_value_2
                  (bind (_outcell_2 _returnvalue_3) (`GridManager.TryGetGridCell` _grid_manager_2 _grid_coord_2))
                  (if _returnvalue_3
                    (bind (_coord _bblocked _movecost _movecostlistindex _bisoccupied) (break `GridCell` _outcell_2))
                    (if _bblocked
                      (`KismetSystemLibrary.PrintString` "Cannot move unit: target cell is blocked or occupied." :!label _label)
                      (elif _bisoccupied
                        (goto _label)
                        (else
                          ; Unit Movement Logic
                          (`self.Selected Character`
                            (:`then`
                              (`/Game/Blueprint/Character/BP_TacticalCharacter.Start Move Along Path` :`self` (`self.Selected Character`) :`Grid Manager` (`self.Grid Manager`))
                              (set `self.Interaction Lock` true))
                            (:`else`))))))))
              (:`else`))))))))

(event `EnhancedInput|/Game/Input/InputActions/IA_SwitchMode`
  (params (ActionValue :type Boolean) (ElapsedSeconds :type "Float (double-precision)") (TriggeredSeconds :type "Float (double-precision)") (InputAction :type "InputAction Object Reference" :default "/Game/Input/InputActions/IA_SwitchMode.IA_SwitchMode"))
  (:`Triggered`
    (`self.Interaction Lock`
      (:`then`)
      (:`else`
        (switch `/Game/Blueprint/Enum/E_WeightedTerrianMode` (`self.Current Mode`)
          (:`NewEnumerator0`
            (set `self.Current Mode` "NewEnumerator1")
            (bind _grid_manager (`self.Grid Manager`)
              (:`then`
                (set `GridManager.bEnableHoverPathPreview` true _grid_manager)
                (`GridManager.RemoveStartAndGoalCoord` _grid_manager)
                (set `GridManager.bEnableAbilityPreview` false _grid_manager)
                (set `TextBlock.Text` "Movement Range" (`/Game/UI/W_TooltipTacticalMovement.ModeName` (`self.UI`))))
              (:`else`)))
          (:`NewEnumerator1`
            (set `self.Current Mode` "NewEnumerator2")
            (bind _grid_manager_2 (`self.Grid Manager`)
              (:`then`
                (set `GridManager.bEnableHoverPathPreview` false _grid_manager_2)
                (`GridManager.RemoveStartAndGoalCoord` _grid_manager_2)
                (set `GridManager.bEnableAbilityPreview` true _grid_manager_2)
                (set `TextBlock.Text` "Ability Attack" (`/Game/UI/W_TooltipTacticalMovement.ModeName` (`self.UI`))))
              (:`else`)))
          (:`NewEnumerator2`
            (set `self.Current Mode` "NewEnumerator0")
            (bind _grid_manager_3 (`self.Grid Manager`)
              (:`then`
                (set `GridManager.bEnableHoverPathPreview` false _grid_manager_3)
                (`GridManager.RemoveStartAndGoalCoord` _grid_manager_3)
                (set `GridManager.bEnableAbilityPreview` false _grid_manager_3)
                (set `TextBlock.Text` "Terrain Editor" (`/Game/UI/W_TooltipTacticalMovement.ModeName` (`self.UI`))))
              (:`else`))))))))

(event `self.ReceiveTick`
  (params (DeltaSeconds :type "Float (single-precision)"))
  (bind _current_skill (`self.Current Skill`))
  (bind (_returnvalue_x _returnvalue_y) (`KismetMathLibrary.BreakVector` (`SceneComponent.K2_GetComponentLocation` (`Character.CapsuleComponent` (`self.Selected Character`)))))
  (bind (_returnvalue_x_2 _returnvalue_y_2 _returnvalue_z) (`KismetMathLibrary.BreakVector` (`SceneComponent.K2_GetComponentLocation` (`GridManager.SceneRoot` (`self.Grid Manager`)))))
  (if (`|EnumEquality` (`self.Current Mode`) "NewEnumerator2")
    (bind _selected_character (`self.Selected Character`)
      (:`then`
        (bind _character_preset (`/Game/Blueprint/Character/BP_TacticalCharacter.Character Preset` _selected_character)
          (:`then`
            (bind _output (`|GetArrayItem` (`/Game/Blueprint/DataAsset/Unit/DA_Unit.Skill Preset` _character_preset)))
            (`/Engine/EditorBlueprintResources/StandardMacros.IsValid` _output
              (:`Is Valid`
                (set `self.Current Skill` _output)
                ; Ability Origin Coord
                (set `self.Origin Coord` (`GridManager.WorldToGrid` (`self.Grid Manager`) (`KismetMathLibrary.MakeVector` _returnvalue_x _returnvalue_y _returnvalue_z)))
                ; Get hovered grid, ability target coord
                (`self.Grid Manager`
                  (:`then`
                    (bind (_grid_coord _return_value) (`self.Run Raytrace`))
                    (if _return_value
                      (set `self.Hover Coord` _grid_coord)
                      (`GridManager.UpdateAbilityPreview` (`self.Grid Manager`) (`self.Origin Coord`) (`self.Hover Coord`) (`KismetMathLibrary.FTrunc` (`/Game/Blueprint/DataAsset/Skill/DA_Skill.Attack Range` _current_skill)) (`KismetMathLibrary.FTrunc` (`/Game/Blueprint/DataAsset/Skill/DA_Skill.Effect Range` _current_skill)))))
                  (:`else`)))))
          (:`else`)))
      (:`else`))))

(fn `Run Findpath`
  (returns (`Path Is Valid` :type Boolean))
  (bind _grid_manager (`self.Grid Manager`)
    (:`then`
      (bind _returnvalue (`GridManager.FindPath` _grid_manager))
      (return _returnvalue))
    (:`else`)))

(fn `Run Raytrace`
  (returns (`Grid Coord` :type "GridCoord Structure") (`Return Value` :type Boolean))
  (bind (_locationx _locationy) (`self.GetMousePosition`))
  (bind (_worldposition _worlddirection) (`GameplayStatics.DeprojectScreenToWorld` self (`KismetMathLibrary.MakeVector2D` _locationx _locationy)))
  (`self.Grid Manager`
    (:`then`
      (bind (_outhit _returnvalue) (`KismetSystemLibrary.LineTraceSingle` _worldposition (+ _worldposition (* _worlddirection (`GridManager.TraceDistance` (`self.Grid Manager`)))) "TraceTypeQuery1"))
      (if _returnvalue
        (return (`GridManager.WorldToGrid` (`self.Grid Manager`) (`KismetMathLibrary.MakeVector` (.x (`.Location` (`GameplayStatics.BreakHitResult` _outhit))) (.y (`.Location` (`GameplayStatics.BreakHitResult` _outhit))))) true)
        (else
          (return (struct) false))))
    (:`else`)))

(fn `UserConstructionScript`)