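; Player controller for a weighted-terrain grid scene, switching between Terrain Editor and Movement Range modes.
; On begin play it sets up Enhanced Input, configures the GridManager to draw cell costs and creates a tooltip widget showing the mode.
; Left click line-traces from the cursor to a grid coord, then cycles that cell's cost or sets the start coord.
; Switching modes clears start and goal and toggles hover path preview.
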(event `self.ReceiveBeginPlay`
  (bind _returnvalue (subsystem `EnhancedInputLocalPlayerSubsystem`))
  (`|ExecutionSequence`
    (:`then_0`
      (set `self.bShowMouseCursor` true)
      (bind _asbp_grid_pawn (cast `/Game/Blueprint/Pawn/BP_GridPawn` (`self.K2_GetPawn`)))
      (set `self.Controlled Pawn` _asbp_grid_pawn)
      (`/Engine/EditorBlueprintResources/StandardMacros.IsValid` _returnvalue
        (:`Is Valid`
          (`EnhancedInputSubsystemInterface.AddMappingContext` _returnvalue "/Game/Input/IMC_Grid.IMC_Grid" 0 (struct))
          (bind _returnvalue_2 (`GameplayStatics.GetActorOfClass` "/Script/GridExperiment.GridManager"))
          (`/Engine/EditorBlueprintResources/StandardMacros.IsValid` _returnvalue_2
            (:`Is Valid`
              (bind _output_get (set `self.Grid Manager` _returnvalue_2))
              (set `GridManager.bDrawCellCostText` true _output_get)
              (set `GridManager.bEnableAbilityPreview` false _output_get))))))
    (:`then_1`
      (bind _returnvalue_3 (`|CreateWidget` "/Game/UI/W_TooltipWeightedTerrain.W_TooltipWeightedTerrain_C"))
      (`UserWidget.AddToViewport` _returnvalue_3 0)
      (set `self.UI` _returnvalue_3))))

(event `EnhancedInput|/Game/Input/InputActions/IA_GridMove`
  (params (ActionValue :type "Vector2D Structure") (ElapsedSeconds :type "Float (double-precision)") (TriggeredSeconds :type "Float (double-precision)") (InputAction :type "InputAction Object Reference" :default "/Game/Input/InputActions/IA_GridMove.IA_GridMove"))
  (:`Triggered`
    ;[0.15 0.15 0.15 0.502] Camera Logic
    (`Pawn.AddMovementInput` (`self.Controlled Pawn`) (`self.Right Unit`) ActionValue_X false)
    (`Pawn.AddMovementInput` (`self.Controlled Pawn`) (`self.Up Unit`) ActionValue_Y false)))

(event `EnhancedInput|/Game/Input/InputActions/IA_GridLeft`
  (params (ActionValue :type Boolean) (ElapsedSeconds :type "Float (double-precision)") (TriggeredSeconds :type "Float (double-precision)") (InputAction :type "InputAction Object Reference" :default "/Game/Input/InputActions/IA_GridLeft.IA_GridLeft"))
  (:`Triggered`
    (switch `/Game/Blueprint/Enum/E_WeightedTerrianMode` (`self.Current Mode`)
      (:`NewEnumerator0`
        ; Get clicked grid and validate
        (bind _grid_manager (`self.Grid Manager`)
          (:`then`
            (bind (_grid_coord _return_value) (`self.Run Raytrace`))
            (if _return_value
              (if (`GridManager.IsValidCoord` _grid_manager _grid_coord)
                ; Perform grid operation
                (`GridManager.CycleGridCost` _grid_manager _grid_coord))))
          (:`else`)))
      (:`NewEnumerator1`
        ; Get clicked grid and validate
        (bind _grid_manager_2 (`self.Grid Manager`)
          (:`then`
            (bind (_grid_coord_2 _return_value_2) (`self.Run Raytrace`))
            (if _return_value_2
              (if (`GridManager.IsValidCoord` _grid_manager_2 _grid_coord_2)
                (`GridManager.SetStartCoord` _grid_manager_2 _grid_coord_2))))
          (:`else`))))))

(event `EnhancedInput|/Game/Input/InputActions/IA_SwitchMode`
  (params (ActionValue :type Boolean) (ElapsedSeconds :type "Float (double-precision)") (TriggeredSeconds :type "Float (double-precision)") (InputAction :type "InputAction Object Reference" :default "/Game/Input/InputActions/IA_SwitchMode.IA_SwitchMode"))
  (:`Triggered`
    (if (`|EnumEquality` (`self.Current Mode`) "NewEnumerator0")
      (set `self.Current Mode` "NewEnumerator1")
      (bind _grid_manager (`self.Grid Manager`)
        (:`then`
          (set `GridManager.bEnableHoverPathPreview` true _grid_manager)
          (`GridManager.RemoveStartAndGoalCoord` _grid_manager)
          (set `TextBlock.Text` "Movement Range" (`/Game/UI/W_TooltipWeightedTerrain.ModeName` (`self.UI`))))
        (:`else`))
      (else
        (set `self.Current Mode` "NewEnumerator0")
        (bind _grid_manager_2 (`self.Grid Manager`)
          (:`then`
            (set `GridManager.bEnableHoverPathPreview` false _grid_manager_2)
            (`GridManager.RemoveStartAndGoalCoord` _grid_manager_2)
            (set `TextBlock.Text` "Terrain Editor" (`/Game/UI/W_TooltipWeightedTerrain.ModeName` (`self.UI`))))
          (:`else`))))))

(fn `Run Findpath`
  (returns (`Path Is Valid` :type Boolean))
  (bind _grid_manager (`self.Grid Manager`)
    (:`then`
      (bind _returnvalue (`GridManager.FindPath` _grid_manager))
      (return _returnvalue))
    (:`else`)))

(fn `Run Raytrace`
  (returns (`Grid Coord` :type "GridCoord Structure") (`Return Value` :type Boolean))
  (bind (_locationx _locationy) (`self.GetMousePosition`))
  (bind (_worldposition _worlddirection) (`GameplayStatics.DeprojectScreenToWorld` self (`KismetMathLibrary.MakeVector2D` _locationx _locationy)))
  (`self.Grid Manager`
    (:`then`
      (bind (_outhit _returnvalue) (`KismetSystemLibrary.LineTraceSingle` _worldposition (+ _worldposition (* _worlddirection (`GridManager.TraceDistance` (`self.Grid Manager`)))) "TraceTypeQuery1"))
      (if _returnvalue
        (return (`GridManager.WorldToGrid` (`self.Grid Manager`) (`KismetMathLibrary.MakeVector` (.x (`.Location` (`GameplayStatics.BreakHitResult` _outhit))) (.y (`.Location` (`GameplayStatics.BreakHitResult` _outhit))))) true)
        (else
          (return (struct) false))))
    (:`else`)))

(fn `UserConstructionScript`)